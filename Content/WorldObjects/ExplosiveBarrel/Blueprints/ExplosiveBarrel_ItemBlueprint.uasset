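; Explosive barrel world object, drawn with a Paper2D flipbook, that blows up when it takes any damage.
; The first hit, gated by a DoOnce, spawns the separate explosion Blueprint at the flipbook's transform and destroys the barrel.
; Every tick it sets its yaw toward player 0's character, so the flat sprite acts as a yaw-only billboard.
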(event Game|Damage|EventAnyDamage
  (params (Damage :type Float%20%28single-precision%29) (DamageType :type Damage%20Type%20Object%20Reference) (InstigatedBy :type Controller%20Object%20Reference) (DamageCauser :type Actor%20Object%20Reference))
  ;[1 1 1] Spawn Explosion When Barrel Takes Damage
  (Utilities|FlowControl|DoOnce false
    (:Completed
      (Game|SpawnActorfromClass "/Game/WorldObjects/ExplosiveBarrel/Blueprints/ExplosiveBarrel_ExplosionBlueprint.ExplosiveBarrel_ExplosionBlueprint_C" (Transformation|GetWorldTransform (Variables|Default|GetPaperFlipbook)) "Undefined" 0 0)
      (Actor|DestroyActor))))

(event EventTick
  (params (DeltaSeconds :type Float%20%28single-precision%29))
  ;[1 1 1] Event Tick Yaw Rotations
  (Transformation|SetActorRotation (Math|Rotator|MakeRotator 0.0 0.0 (.yaw (Math|Rotator|FindLookatRotation (Transformation|GetActorLocation) (Transformation|GetActorLocation (Game|GetPlayerCharacter 0)))))))

(fn ConstructionScript)