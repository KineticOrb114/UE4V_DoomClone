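; Axe melee weapon Blueprint, animated with Paper2D flipbooks on a shared weapon base.
; Attack runs behind a DoOnce gate: it swaps to the attack flipbook, calls MeleeAttack and plays a 2D sound.
; After a short delay it restores the idle flipbook and reopens the gate, limiting the attack rate.
; BeginPlay copies the first-person character's ammo counts for every gun type into the weapon's ammo variables.
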(event EventBeginPlay
  ;[1 1 1] Set BaseWeapon Ammo
  (bind _asfirst_person_character (Utilities|Casting|CastToFirstPersonCharacter (Game|GetPlayerCharacter 0)))
  (Variables|Default|SetPistolAmmo (Variables|/Game/FirstPersonBP/Blueprints/FirstPersonCharacter.FirstPersonCharacter_C|GetFpcPistolAmmo _asfirst_person_character))
  (Variables|Default|SetShotgunAmmo (Variables|/Game/FirstPersonBP/Blueprints/FirstPersonCharacter.FirstPersonCharacter_C|GetFpcShotgunAmmo _asfirst_person_character))
  (Variables|Default|SetUziAmmo (Variables|/Game/FirstPersonBP/Blueprints/FirstPersonCharacter.FirstPersonCharacter_C|GetFpcUziAmmo _asfirst_person_character))
  (Variables|Default|SetMinigunAmmo (Variables|/Game/FirstPersonBP/Blueprints/FirstPersonCharacter.FirstPersonCharacter_C|GetFpcMinigunAmmo _asfirst_person_character))
  (Variables|Default|SetRpgAmmo (Variables|/Game/FirstPersonBP/Blueprints/FirstPersonCharacter.FirstPersonCharacter_C|GetFpcRpgAmmo _asfirst_person_character)))

(event EventAttack
  ;[1 1 1] Attack
  (Utilities|FlowControl|DoOnce false :!label _label
    (:Completed
      (Sprite|SetFlipbook (Variables|Default|GetPaperFlipbook) "/Game/Guns/Axe/Flipbooks/Axe_AttackFlipbook.Axe_AttackFlipbook")
      (CallFunction|MeleeAttack)
      (Audio|PlaySound2D "/Game/Sounds/Axe_SoundWave.Axe_SoundWave" 1.0 1.0 0.0 0 0)
      (Utilities|FlowControl|Delay 0.2)
      (Sprite|SetFlipbook (Variables|Default|GetPaperFlipbook) "/Game/Guns/Axe/Flipbooks/Axe_IdleFlipbook.Axe_IdleFlipbook")
      (goto _label Reset))))

(fn ConstructionScript
  (|CallParentFunction))