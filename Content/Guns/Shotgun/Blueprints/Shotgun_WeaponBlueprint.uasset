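; Shotgun weapon Blueprint, built on a base weapon, that fires with a flipbook sprite animation and sound.
; On BeginPlay it copies all five ammo counts from the FirstPersonCharacter.
; Attack uses a DoOnce gate: with shells left it decrements shotgun ammo, plays the fire flipbook, calls Fire and plays the sound.
; A short delay then restores the idle flipbook and reopens the gate, capping fire rate.
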(event EventBeginPlay
  ;[1 1 1] Set BaseWeapon Ammo
  (bind _asfirst_person_character (Utilities|Casting|CastToFirstPersonCharacter (Game|GetPlayerCharacter 0)))
  (Variables|Default|SetPistolAmmo (Variables|/Game/FirstPersonBP/Blueprints/FirstPersonCharacter.FirstPersonCharacter_C|GetFpcPistolAmmo _asfirst_person_character))
  (Variables|Default|SetShotgunAmmo (Variables|/Game/FirstPersonBP/Blueprints/FirstPersonCharacter.FirstPersonCharacter_C|GetFpcShotgunAmmo _asfirst_person_character))
  (Variables|Default|SetUziAmmo (Variables|/Game/FirstPersonBP/Blueprints/FirstPersonCharacter.FirstPersonCharacter_C|GetFpcUziAmmo _asfirst_person_character))
  (Variables|Default|SetMinigunAmmo (Variables|/Game/FirstPersonBP/Blueprints/FirstPersonCharacter.FirstPersonCharacter_C|GetFpcMinigunAmmo _asfirst_person_character))
  (Variables|Default|SetRpgAmmo (Variables|/Game/FirstPersonBP/Blueprints/FirstPersonCharacter.FirstPersonCharacter_C|GetFpcRpgAmmo _asfirst_person_character)))

(event EventAttack
  (bind _shotgunammo (Variables|Default|GetShotgunAmmo))
  ;[1 1 1] Attack
  (Utilities|FlowControl|DoOnce false :!label _label
    (:Completed
      (if (> _shotgunammo 0.0)
        (Math|Float|DecrementFloat _shotgunammo
          (:%20%20
            (Sprite|SetFlipbook (Variables|Default|GetPaperFlipbook) "/Game/Guns/Shotgun/Flipbooks/Shotgun_FireFlipbook.Shotgun_FireFlipbook")
            (CallFunction|Fire)
            (Audio|PlaySound2D "/Game/Sounds/Shotgun_SoundWave.Shotgun_SoundWave" 1.0 1.0 0.0 0 0)
            (Utilities|FlowControl|Delay 0.6)
            (Sprite|SetFlipbook (Variables|Default|GetPaperFlipbook) "/Game/Guns/Shotgun/Flipbooks/Shotgun_IdleFlipbook.Shotgun_IdleFlipbook")
            (goto _label Reset)))
        (else
          (goto _label Reset))))))

(fn ConstructionScript
  (|CallParentFunction))