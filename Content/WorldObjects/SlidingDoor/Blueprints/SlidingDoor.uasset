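; Sliding door actor that opens upward once when the first-person character enters its Box trigger, then removes itself.
; A DoOnce-gated overlap plays a 2D open sound and starts a timeline.
; Each timeline update raises the mesh's world Z by lerping from its current height, so movement accumulates per tick.
; A 1.5-second delay, triggered from the update pin, ends in destroying the actor.
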(event OnComponentBeginOverlap(Box)
  (params (OverlappedComponent :type Primitive%20Component%20Object%20Reference) (OtherActor :type Actor%20Object%20Reference) (OtherComp :type Primitive%20Component%20Object%20Reference) (OtherBodyIndex :type Integer) (bFromSweep :type Boolean) (SweepResult :type Hit%20Result%20Structure%20%28by%20ref%29))
  (bind _staticmesh (Variables|Default|GetStaticMesh))
  (bind _returnvalue (Transformation|GetWorldLocation _staticmesh))
  ;[1 1 1] Move Door on Box Collision
  (Utilities|Casting|CastToFirstPersonCharacter OtherActor)
  (Utilities|FlowControl|DoOnce false
    (:Completed
      (Audio|PlaySound2D "/Game/Sounds/DoorOpen_SoundWave.DoorOpen_SoundWave" 1.0 1.0 0.0 0 0)
      (bind _newtrack_0 (Timeline|SlidingDoor_OpenTimeline PlayFromStart)
        (:Update
          (Transformation|SetWorldLocation _staticmesh (Math|Vector|MakeVector (.x _returnvalue) (.y _returnvalue) (Math|Float|Lerp (.z _returnvalue) (+ (.z _returnvalue) 4e+01) _newtrack_0)) false false)
          (Utilities|FlowControl|Delay 1.5)
          (Actor|DestroyActor))))))

(fn ConstructionScript)