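; RPG weapon Blueprint, a child weapon that fires rockets with flipbook sprite animation for the first-person character.
; On BeginPlay it copies the ammo counts for every weapon type from the player character.
; Attack spends one RPG round, calls FireRpg, plays the launch sound and steps through fire, after-fire and idle flipbooks.
; A DoOnce gate, reset after the timed delays, limits the fire rate.
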(event EventBeginPlay
  ;[1 1 1] Set BaseWeapon Ammo
  (bind _asfirst_person_character (Utilities|Casting|CastToFirstPersonCharacter (Game|GetPlayerCharacter 0)))
  (Variables|Default|SetPistolAmmo (Variables|/Game/FirstPersonBP/Blueprints/FirstPersonCharacter.FirstPersonCharacter_C|GetFpcPistolAmmo _asfirst_person_character))
  (Variables|Default|SetShotgunAmmo (Variables|/Game/FirstPersonBP/Blueprints/FirstPersonCharacter.FirstPersonCharacter_C|GetFpcShotgunAmmo _asfirst_person_character))
  (Variables|Default|SetUziAmmo (Variables|/Game/FirstPersonBP/Blueprints/FirstPersonCharacter.FirstPersonCharacter_C|GetFpcUziAmmo _asfirst_person_character))
  (Variables|Default|SetMinigunAmmo (Variables|/Game/FirstPersonBP/Blueprints/FirstPersonCharacter.FirstPersonCharacter_C|GetFpcMinigunAmmo _asfirst_person_character))
  (Variables|Default|SetRpgAmmo (Variables|/Game/FirstPersonBP/Blueprints/FirstPersonCharacter.FirstPersonCharacter_C|GetFpcRpgAmmo _asfirst_person_character)))

(event EventAttack
  (bind _rpgammo (Variables|Default|GetRpgAmmo))
  ;[1 1 1] Attack
  (Utilities|FlowControl|DoOnce false :!label _label
    (:Completed
      (if (> _rpgammo 0.0)
        (Math|Float|DecrementFloat _rpgammo
          (:%20%20
            (CallFunction|FireRpg)
            (Audio|PlaySound2D "/Game/Sounds/Launcher_SoundWave.Launcher_SoundWave" 1.0 1.0 0.0 0 0)
            (Sprite|SetFlipbook (Variables|Default|GetPaperFlipbook) "/Game/Guns/RPG/Flipbooks/Rpg_FireFlipbook.Rpg_FireFlipbook")
            (Utilities|FlowControl|Delay 0.2)
            (Sprite|SetFlipbook (Variables|Default|GetPaperFlipbook) "/Game/Guns/RPG/Flipbooks/Rpg_AfterFlipbook.Rpg_AfterFlipbook")
            (Utilities|FlowControl|Delay 0.8)
            (Sprite|SetFlipbook (Variables|Default|GetPaperFlipbook) "/Game/Guns/RPG/Flipbooks/Rpg_IdleFlipbook.Rpg_IdleFlipbook")
            (goto _label Reset)))
        (else
          (goto _label Reset))))))

(fn ConstructionScript
  (|CallParentFunction))