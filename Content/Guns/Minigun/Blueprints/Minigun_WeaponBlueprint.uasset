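; Minigun weapon Blueprint, a child weapon with Paper2D flipbook visuals that fires automatically while attack is held.
; Attack starts a looping timer that calls the inherited Fire, plays sound and fire flipbook, and spends ammo each tick.
; AttackStop or empty ammo clears the fire flag and restores the idle flipbook, without clearing the timer.
; BeginPlay copies ammo counts for all weapon types from the first-person character.
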(event Custom|FireMinigun
  ;[1 1 1] Attack / AttackStop
  (if (> (Variables|Default|GetMinigunAmmo) 0.0)
    (if (Variables|Default|GetShouldFire)
      (Sprite|SetFlipbook (Variables|Default|GetPaperFlipbook) "/Game/Guns/Minigun/Flipbooks/Minigun_FireFlipbook.Minigun_FireFlipbook")
      (CallFunction|Fire)
      (Audio|PlaySound2D "/Game/Sounds/MiniGun_SW.MiniGun_SW" 1.0 1.0 0.0 0 0)
      (Math|Float|DecrementFloat (Variables|Default|GetMinigunAmmo)))
    (else
      (Variables|Default|SetShouldFire false)
      (Sprite|SetFlipbook (Variables|Default|GetPaperFlipbook) "/Game/Guns/Minigun/Flipbooks/Minigun_IdleFlipbook.Minigun_IdleFlipbook"))))

(event EventBeginPlay
  ;[1 1 1] Set BaseWeapon Ammo
  (bind _asfirst_person_character (Utilities|Casting|CastToFirstPersonCharacter (Game|GetPlayerCharacter 0)))
  (Variables|Default|SetPistolAmmo (Variables|/Game/FirstPersonBP/Blueprints/FirstPersonCharacter.FirstPersonCharacter_C|GetFpcPistolAmmo _asfirst_person_character))
  (Variables|Default|SetShotgunAmmo (Variables|/Game/FirstPersonBP/Blueprints/FirstPersonCharacter.FirstPersonCharacter_C|GetFpcShotgunAmmo _asfirst_person_character))
  (Variables|Default|SetUziAmmo (Variables|/Game/FirstPersonBP/Blueprints/FirstPersonCharacter.FirstPersonCharacter_C|GetFpcUziAmmo _asfirst_person_character))
  (Variables|Default|SetMinigunAmmo (Variables|/Game/FirstPersonBP/Blueprints/FirstPersonCharacter.FirstPersonCharacter_C|GetFpcMinigunAmmo _asfirst_person_character))
  (Variables|Default|SetRpgAmmo (Variables|/Game/FirstPersonBP/Blueprints/FirstPersonCharacter.FirstPersonCharacter_C|GetFpcRpgAmmo _asfirst_person_character)))

(event EventAttack
  ;[1 1 1] Attack / AttackStop
  (Variables|Default|SetShouldFire true)
  (Utilities|Time|SetTimerbyEvent (delegate Custom|FireMinigun) 0.1 true))

(event EventAttackStop
  ;[1 1 1] Attack / AttackStop
  (Variables|Default|SetShouldFire false)
  (Sprite|SetFlipbook (Variables|Default|GetPaperFlipbook) "/Game/Guns/Minigun/Flipbooks/Minigun_IdleFlipbook.Minigun_IdleFlipbook"))

(fn ConstructionScript
  (|CallParentFunction))