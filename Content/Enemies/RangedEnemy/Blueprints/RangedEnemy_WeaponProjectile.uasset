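; Projectile actor for the ranged enemy's weapon that damages the first-person player on contact.
; Each tick it sets its yaw to face player character 0.
; A sphere overlap with the FirstPersonCharacter applies a small fixed damage and destroys the projectile.
; A delay started on BeginPlay destroys it after ten seconds if it hits nothing.
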(event OnComponentBeginOverlap(Sphere)
  (params (OverlappedComponent :type Primitive%20Component%20Object%20Reference) (OtherActor :type Actor%20Object%20Reference) (OtherComp :type Primitive%20Component%20Object%20Reference) (OtherBodyIndex :type Integer) (bFromSweep :type Boolean) (SweepResult :type Hit%20Result%20Structure%20%28by%20ref%29))
  ;[1 1 1] On Component Begin Overlap
  (bind _asfirst_person_character (Utilities|Casting|CastToFirstPersonCharacter OtherActor))
  (Game|Damage|ApplyDamage _asfirst_person_character 2.0 0 0)
  (Actor|DestroyActor))

(event EventBeginPlay
  ;[1 1 1] DestroyActor Without Collision
  (Utilities|FlowControl|Delay 1e+01)
  (Actor|DestroyActor))

(event EventTick
  (params (DeltaSeconds :type Float%20%28single-precision%29))
  ;[1 1 1] Event Tick Yaw Rotations
  (Transformation|SetActorRotation (Math|Rotator|MakeRotator 0.0 0.0 (.yaw (Math|Rotator|FindLookatRotation (Transformation|GetActorLocation) (Transformation|GetActorLocation (Game|GetPlayerCharacter 0)))))))

(fn ConstructionScript)