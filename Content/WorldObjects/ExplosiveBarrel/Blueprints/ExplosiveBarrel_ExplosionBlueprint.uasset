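; Explosion actor for the explosive barrel that damages actors and removes itself after a brief lifetime.
; On BeginPlay it plays a 2D explosion sound, then destroys itself after a short delay.
; Any actor that begins overlapping its sphere during that window receives a fixed amount of damage.
; Each tick it turns its yaw toward the player pawn, billboard-style.
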(event OnComponentBeginOverlap(Sphere)
  (params (OverlappedComponent :type Primitive%20Component%20Object%20Reference) (OtherActor :type Actor%20Object%20Reference) (OtherComp :type Primitive%20Component%20Object%20Reference) (OtherBodyIndex :type Integer) (bFromSweep :type Boolean) (SweepResult :type Hit%20Result%20Structure%20%28by%20ref%29))
  ;[1 1 1] Apply Damage to Other Actor
  (Game|Damage|ApplyDamage OtherActor 1e+01 0 0))

(event EventBeginPlay
  ;[1 1 1] Trigger Sound Before DestroyActor
  (Audio|PlaySound2D "/Game/Sounds/Explosion_SoundWave.Explosion_SoundWave" 1.0 1.0 0.0 0 0)
  (Utilities|FlowControl|Delay 0.5)
  (Actor|DestroyActor))

(event EventTick
  (params (DeltaSeconds :type Float%20%28single-precision%29))
  ;[1 1 1] Event Tick Yaw Rotations
  (Transformation|SetActorRotation (Math|Rotator|MakeRotator 0.0 0.0 (.yaw (Math|Rotator|FindLookatRotation (Transformation|GetActorLocation) (Transformation|GetActorLocation (Game|Player|GetPlayerPawn 0)))))))

(fn ConstructionScript)