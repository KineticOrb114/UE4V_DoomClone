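; Pistol ammo pickup that adds rounds to the player's weapon when the first-person character overlaps its box.
; Each tick it turns on yaw only to face the player.
; On overlap it casts to the character and its weapon child actor, then adds a fixed, clamped amount to PistolAmmo.
; It destroys itself only when ammo was below the cap, so it stays in place otherwise.
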(event OnComponentBeginOverlap(Box)
  (params (OverlappedComponent :type Primitive%20Component%20Object%20Reference) (OtherActor :type Actor%20Object%20Reference) (OtherComp :type Primitive%20Component%20Object%20Reference) (OtherBodyIndex :type Integer) (bFromSweep :type Boolean) (SweepResult :type Hit%20Result%20Structure%20%28by%20ref%29))
  ;[1 1 1] HealthPickup Box Collision
  (bind _asfirst_person_character (Utilities|Casting|CastToFirstPersonCharacter OtherActor))
  (bind _asbase_weapon_blueprint (Utilities|Casting|CastToBase_WeaponBlueprint (Variables|/Script/Engine.ChildActorComponent|GetChildActor (Variables|/Game/FirstPersonBP/Blueprints/FirstPersonCharacter.FirstPersonCharacter_C|GetWeapon _asfirst_person_character))))
  (if (< (Variables|/Game/Guns/Base/Blueprints/Base_WeaponBlueprint.Base_WeaponBlueprint_C|GetPistolAmmo _asbase_weapon_blueprint) 5e+01)
    (Variables|/Game/Guns/Base/Blueprints/Base_WeaponBlueprint.Base_WeaponBlueprint_C|SetPistolAmmo _asbase_weapon_blueprint (Math|Float|Clamp(Float) (+ (Variables|/Game/Guns/Base/Blueprints/Base_WeaponBlueprint.Base_WeaponBlueprint_C|GetPistolAmmo _asbase_weapon_blueprint) 5.0) 0.0 5e+01))
    (Actor|DestroyActor)))

(event EventTick
  (params (DeltaSeconds :type Float%20%28single-precision%29))
  ;[1 1 1] EventTick Yaw Rotations
  (Transformation|SetActorRotation (Math|Rotator|MakeRotator 0.0 0.0 (.yaw (Math|Rotator|FindLookatRotation (Transformation|GetActorLocation) (Transformation|GetActorLocation (Game|GetPlayerCharacter 0)))))))

(fn ConstructionScript)