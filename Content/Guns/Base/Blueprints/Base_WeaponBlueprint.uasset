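; Base weapon Blueprint that provides shared hitscan, rocket and melee attack functions, with empty Attack and AttackStop events.
; Fire line-traces forward from WeaponTrace and applies gun damage if any pistol, shotgun, Uzi or minigun ammo remains.
; FireRpg checks RPG ammo and spawns a projectile at WeaponTrace, while MeleeAttack uses a short pawn-only trace to apply melee damage.
; None of these functions decrements ammo, and both traces draw debug lines.
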(event Custom|Attack)

(event Custom|AttackStop)

(fn ConstructionScript)

(fn Fire
  (bind _weapontrace (Variables|Default|GetWeaponTrace))
  (bind _returnvalue (Transformation|GetWorldLocation _weapontrace))
  ;[1 1 1] Fire
  (if (Math|Boolean|ORBoolean (> (Variables|Default|GetPistolAmmo) 0.0) (> (Variables|Default|GetShotgunAmmo) 0.0) (> (Variables|Default|GetUziAmmo) 0.0) (> (Variables|Default|GetMinigunAmmo) 0.0))
    (bind (_outhit _returnvalue_2) (Collision|LineTraceForObjects _returnvalue (+ _returnvalue (* (Math|Vector|GetForwardVector (Transformation|GetWorldRotation _weapontrace)) 4e+03)) (Utilities|Array|MakeArray "ObjectTypeQuery3" "ObjectTypeQuery1") false 0 "ForDuration"))
    (if _returnvalue_2
      (Game|Damage|ApplyDamage (.HitActor (Collision|BreakHitResult _outhit)) (Variables|Default|GetGunDamage) 0 0))))

(fn FireRpg
  ;[1 1 1] Fire Rpg
  (if (> (Variables|Default|GetRpgAmmo) -1.0)
    (Game|SpawnActorfromClass "/Game/Guns/RPG/Blueprints/Rpg_ProjectileBlueprint.Rpg_ProjectileBlueprint_C" (Transformation|GetWorldTransform (Variables|Default|GetWeaponTrace)) "Undefined" 0 0)))

(fn MeleeAttack
  (bind _weapontrace (Variables|Default|GetWeaponTrace))
  (bind _returnvalue (Transformation|GetWorldLocation _weapontrace))
  ;[1 1 1] Melee Attack
  (bind (_outhit _returnvalue_2) (Collision|LineTraceForObjects _returnvalue (+ _returnvalue (* (Math|Vector|GetForwardVector (Transformation|GetWorldRotation _weapontrace)) 5e+01)) (Utilities|Array|MakeArray "ObjectTypeQuery3") false 0 "ForDuration"))
  (if _returnvalue_2
    (Game|Damage|ApplyDamage (.HitActor (Collision|BreakHitResult _outhit)) (Variables|Default|GetMeleeDamage) 0 0)))