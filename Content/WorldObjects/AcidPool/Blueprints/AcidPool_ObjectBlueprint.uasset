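; Acid pool world object that damages the player while they stand inside its box trigger.
; Box overlap begin and end events, filtered to FirstPersonCharacter, toggle a flag for whether the player is in the pool.
; A looping timer started on BeginPlay checks that flag at short intervals and applies fixed damage to player character 0 while it is set.
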(event OnComponentBeginOverlap(Box)
  (params (OverlappedComponent :type Primitive%20Component%20Object%20Reference) (OtherActor :type Actor%20Object%20Reference) (OtherComp :type Primitive%20Component%20Object%20Reference) (OtherBodyIndex :type Integer) (bFromSweep :type Boolean) (SweepResult :type Hit%20Result%20Structure%20%28by%20ref%29))
  ;[1 1 1] IsPlayerAcidPool: True on Component Begin Overlap
  (Utilities|Casting|CastToFirstPersonCharacter OtherActor)
  (Variables|Default|SetIsPlayerAcidPool true))

(event OnComponentEndOverlap(Box)
  (params (OverlappedComponent :type Primitive%20Component%20Object%20Reference) (OtherActor :type Actor%20Object%20Reference) (OtherComp :type Primitive%20Component%20Object%20Reference) (OtherBodyIndex :type Integer))
  ;[1 1 1] IsPlayerAcidPool: False on Component End Overlap
  (Utilities|Casting|CastToFirstPersonCharacter OtherActor)
  (Variables|Default|SetIsPlayerAcidPool false))

(event Custom|ApplyAcidDamage
  ;[1 1 1] Apply Acid Damage
  (if (Variables|Default|GetIsPlayerAcidPool)
    (Game|Damage|ApplyDamage (Game|GetPlayerCharacter 0) 1e+01 0 0)))

(event EventBeginPlay
  ;[1 1 1] Apply Acid Damage
  (Utilities|Time|SetTimerbyEvent (delegate Custom|ApplyAcidDamage) 0.35 true))

(fn ConstructionScript)