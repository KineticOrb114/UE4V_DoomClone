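; Ranged 2D-sprite enemy that roams or patrols between two points by behavior state, then fires projectiles at the player once seen.
; PawnSensing starts a looping timer that turns it toward the player and alternates shots with short delays.
; Tick picks idle, run or attack flipbooks for four viewing directions using dot products against the player, faking 3D.
; Damage spawns blood effects; death plays flipbooks, then destroys the actor.
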(event OnSeePawn(PawnSensing)
  (params (Pawn :type Pawn%20Object%20Reference))
  ;[1 1 1] Enemy Attack on PawnSensing
  (Utilities|Casting|CastToFirstPersonCharacter Pawn)
  (Variables|Default|SetIsEnemyChase true)
  (Utilities|Time|SetTimerbyEvent (delegate Custom|AttackPlayer) 0.1 true))

(event Custom|RangedEnemyIsDead
  ;[1 1 1] RangedEnemyIsDead
  (Collision|SetCollisionEnabled (Variables|Collision|GetCapsuleComponent) "NoCollision")
  (Transformation|SetActorRotation (Math|Rotator|MakeRotator 0.0 0.0 (.yaw (Math|Rotator|FindLookatRotation (Transformation|GetActorLocation) (Transformation|GetActorLocation (Game|GetPlayerCharacter 0))))))
  (Components|Activation|Deactivate (Variables|Character|GetCharacterMovement))
  (Utilities|FlowControl|DoOnce false
    (:Completed
      (Transformation|SetRelativeRotation (Variables|Default|GetEnemyFlipbook) "0,-90.000000, 0" false false)
      (Sprite|SetFlipbook (Variables|Default|GetEnemyFlipbook) "/Game/Enemies/RangedEnemy/Flipbooks/RangedEnemy_DeathFlipbook.RangedEnemy_DeathFlipbook")
      (Utilities|FlowControl|Delay 0.4)
      (Transformation|AddActorLocalOffset "0, 0,-30.000000" false false)
      (Sprite|SetFlipbook (Variables|Default|GetEnemyFlipbook) "/Game/Enemies/RangedEnemy/Flipbooks/RangedEnemy_DeathIdleFlipbook.RangedEnemy_DeathIdleFlipbook")
      (Utilities|FlowControl|Delay 5.0)
      (Actor|DestroyActor))))

(event Custom|AttackPlayer
  ;[1 1 1] Enemy Attack on PawnSensing
  (if (not (Variables|Default|GetIsEnemyDead))
    (Variables|Default|SetIsEnemyAttack false)
    (Transformation|SetActorRotation (Math|Rotator|MakeRotator 0.0 0.0 (.yaw (Math|Rotator|FindLookatRotation (Transformation|GetActorLocation) (Transformation|GetActorLocation (Game|GetPlayerCharacter 0))))))
    (if (Variables|Default|GetEnemyShouldFire)
      (Variables|Default|SetIsEnemyAttack true)
      (if (not (Variables|Default|GetIsEnemyDead))
        (Game|SpawnActorfromClass "/Game/Enemies/RangedEnemy/Blueprints/RangedEnemy_WeaponProjectile.RangedEnemy_WeaponProjectile_C" (Transformation|GetWorldTransform (Variables|Default|GetProjectileSpawnLocation)) "Undefined" 0 0)
        (Variables|Default|SetEnemyShouldFire false))
      (else
        (Variables|Default|SetIsEnemyAttack false)
        (Utilities|FlowControl|Delay 0.25)
        (Variables|Default|SetEnemyShouldFire true)))))

(event Game|Damage|EventAnyDamage
  (params (Damage :type Float%20%28single-precision%29) (DamageType :type Damage%20Type%20Object%20Reference) (InstigatedBy :type Controller%20Object%20Reference) (DamageCauser :type Actor%20Object%20Reference))
  ;[1 1 1] Apply Damage / Set IsEnemyDead
  (Effects|SpawnEmitterAttached "/Game/Enemies/EnemyBlood/Particles/EnemyBlood_DamageParticle.EnemyBlood_DamageParticle" (Variables|Default|GetEnemyBloodFrontScene) "None")
  (Effects|SpawnEmitterAttached "/Game/Enemies/EnemyBlood/Particles/EnemyBlood_DamageParticle.EnemyBlood_DamageParticle" (Variables|Default|GetEnemyBloodBackScene) "None")
  (Utilities|FlowControl|Sequence
    (:then_0
      (bind _output_get (Variables|Default|SetEnemyHealth (- (Variables|Default|GetEnemyHealth) Damage)))
      (if (<= _output_get 0.0)
        (Variables|Default|SetIsEnemyDead true)))
    (:then_1
      (Utilities|FlowControl|Delay 0.2)
      (Game|SpawnActorfromClass "/Game/Enemies/EnemyBlood/Decals/EnemyBlood_FloorDecal.EnemyBlood_FloorDecal_C" (Transformation|GetWorldTransform (Variables|Character|GetMesh)) "Undefined" 0 0))))

(event EventBeginPlay
  ;[1 1 1] Enemy Movement
  (switch Utilities|FlowControl|Switch|SwitchonRangedEnemy_BehaviorState (Variables|Default|GetEnemyBehaviorState)
    (:NewEnumerator1
      (Utilities|FlowControl|Delay 2.0 :!label _label)
      (if (not (Variables|Default|GetIsEnemyChase))
        (bind _randomlocation (Class|NavigationSystemV1|GetRandomLocationinNavigableRadius (Transformation|GetActorLocation) 1e+03 0 0))
        (AI|AIMoveTo self _randomlocation 0 5.0 false
          (:then
            (goto _label)))))
    (:NewEnumerator2
      (AI|AIMoveTo self "0, 0, 0" (Variables|Default|GetEnemyTargetPoint1) 5.0 false :!label _label_2
        (:OnSuccess
          (Utilities|FlowControl|Delay 3.0)
          (AI|AIMoveTo self "0, 0, 0" (Variables|Default|GetEnemyTargetPoint2) 5.0 false
            (:OnSuccess
              (Utilities|FlowControl|Delay 3.0)
              (goto _label_2))))))))

(event EventTick
  (params (DeltaSeconds :type Float%20%28single-precision%29))
  (bind _returnvalue (Game|GetPlayerCharacter 0))
  (bind _returnvalue_2 (Transformation|GetActorForwardVector))
  (bind _returnvalue_3 (Transformation|GetActorLocation))
  (bind _enemyflipbook (Variables|Default|GetEnemyFlipbook))
  (bind _enemyflipbook_2 (Variables|Default|GetEnemyFlipbook))
  (bind _enemyflipbook_3 (Variables|Default|GetEnemyFlipbook))
  (bind _enemyflipbook_4 (Variables|Default|GetEnemyFlipbook))
  (bind _returnvalue_4 (Transformation|GetActorLocation _returnvalue))
  (bind _returnvalue_5 (- _returnvalue_4 _returnvalue_3))
  (bind _returnvalue_6 (Math|Vector|Normalize _returnvalue_5))
  (bind _returnvalue_7 (Math|Vector|DotProduct _returnvalue_2 _returnvalue_6))
  (bind _returnvalue_8 (Class|KismetMathLibrary|DegAcos _returnvalue_7))
  ;[1 1 1] Event Tick / Set EnemyFlipbookState
  (if (> (Math|Vector|VectorLength (Variables|/Script/Engine.MovementComponent|GetVelocity (Variables|Character|GetCharacterMovement))) 0.0)
    (if (Variables|Default|GetIsEnemyAttack)
      (Variables|Default|SetEnemyFlipbookState "NewEnumerator2")
      (else
        (Variables|Default|SetEnemyFlipbookState "NewEnumerator1")))
    (elif (Variables|Default|GetIsEnemyAttack)
      (Variables|Default|SetEnemyFlipbookState "NewEnumerator2")
      (else
        (Variables|Default|SetEnemyFlipbookState "NewEnumerator0"))))
  ;[1 1 1] Detect Player's Perspective
  (if (Variables|Default|GetIsEnemyDead)
    (CallFunction|RangedEnemyIsDead)
    (elif (< (Math|Vector|DotProduct (Transformation|GetActorRightVector) _returnvalue_6) 0.0)
      (Math|Float|CompareFloat _returnvalue_8 45.0
        (:>
          (Math|Float|CompareFloat _returnvalue_8 135.0 :!label _label
            (:>
              ;[1 1 1] Enemy Back [3]
              (Transformation|SetRelativeRotation _enemyflipbook "0,90.000000, 0" false false :!label _label_2)
              (Sprite|SetFlipbook _enemyflipbook (Utilities|Array|Get(acopy) (Utilities|Select :Index (Variables|Default|GetEnemyFlipbookState) :NewEnumerator0 (Variables|Default|GetEnemyIdleState) :NewEnumerator1 (Variables|Default|GetEnemyRunState) :NewEnumerator2 (Variables|Default|GetEnemyAttackState)) 3)))
            (:==
              (goto _label_2))
            (:<
              ;[1 1 1] Enemy Right [1]
              (Transformation|SetRelativeRotation _enemyflipbook_4 "0, 0, 0" false false)
              (Sprite|SetFlipbook _enemyflipbook_4 (Utilities|Array|Get(acopy) (Utilities|Select :Index (Variables|Default|GetEnemyFlipbookState) :NewEnumerator0 (Variables|Default|GetEnemyIdleState) :NewEnumerator1 (Variables|Default|GetEnemyRunState) :NewEnumerator2 (Variables|Default|GetEnemyAttackState)) 1)))))
        (:==
          (goto _label))
        (:<
          ;[1 1 1] Enemy Front [0]
          (Transformation|SetRelativeRotation _enemyflipbook_3 "0,-90.000000, 0" false false :!label _label_3)
          (Sprite|SetFlipbook _enemyflipbook_3 (Utilities|Array|Get(acopy) (Utilities|Select :Index (Variables|Default|GetEnemyFlipbookState) :NewEnumerator0 (Variables|Default|GetEnemyIdleState) :NewEnumerator1 (Variables|Default|GetEnemyRunState) :NewEnumerator2 (Variables|Default|GetEnemyAttackState))))))
      (else
        (Math|Float|CompareFloat _returnvalue_8 45.0
          (:>
            _)
          (:==
            _)
          (:<
            (goto _label_3)))
        (Math|Float|CompareFloat _returnvalue_8 135.0
          (:>
            (goto _label_2))
          (:==
            (goto _label_2))
          (:<
            ;[1 1 1] Enemy Left [2]
            (Transformation|SetRelativeRotation _enemyflipbook_2 "0,180.000000, 0" false false)
            (Sprite|SetFlipbook _enemyflipbook_2 (Utilities|Array|Get(acopy) (Utilities|Select :Index (Variables|Default|GetEnemyFlipbookState) :NewEnumerator0 (Variables|Default|GetEnemyIdleState) :NewEnumerator1 (Variables|Default|GetEnemyRunState) :NewEnumerator2 (Variables|Default|GetEnemyAttackState)) 2))))))))

(fn ConstructionScript)